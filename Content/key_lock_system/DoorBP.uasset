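; Door Blueprint for a key-and-lock system that opens when a player holding the red key walks into its trigger box.
; Box overlap casts to FirstPersonCharacter and checks GotRedKey, printing a locked or unlocked message.
; An IsDoorAlreadyOpen flag makes it open only once, via a timeline that lerps the Door's relative rotation from its current value toward a -90 yaw.
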(event OnComponentBeginOverlap(Box)
  (params (OverlappedComponent :type Primitive%20Component%20Object%20Reference) (OtherActor :type Actor%20Object%20Reference) (OtherComp :type Primitive%20Component%20Object%20Reference) (OtherBodyIndex :type Integer) (bFromSweep :type Boolean) (SweepResult :type Hit%20Result%20Structure%20%28by%20ref%29))
  (bind _asfirst_person_character (Utilities|Casting|CastToFirstPersonCharacter OtherActor))
  (if (Variables|/Game/FirstPersonBP/Blueprints/FirstPersonCharacter.FirstPersonCharacter_C|GetGotRedKey _asfirst_person_character)
    (if (not (Variables|Default|GetisDoorAlreadyOpen))
      (Variables|Default|SetisDoorAlreadyOpen true)
      (Development|PrintString "Door Unlocked" true true "(R=0.030112,G=0.575000,B=0.060451,A=1.000000)")
      (bind _open_door (Timeline|Open%20Door PlayFromStart)
        (:Update
          (Transformation|SetRelativeRotation (Variables|Default|GetDoor) (Math|Rotator|Lerp(Rotator) (Variables|/Script/Engine.SceneComponent|GetRelativeRotation (Variables|Default|GetDoor)) "0.000000,-90.000000, 0" _open_door true) false false))))
    (else
      (Development|PrintString "Door Locked " true true "(R=1.000000,G=0.038050,B=0.117728,A=1.000000)"))))

(fn ConstructionScript)